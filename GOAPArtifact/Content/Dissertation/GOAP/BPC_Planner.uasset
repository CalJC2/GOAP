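; GOAP planner component that searches for an action sequence taking an AI from its current world state to a goal state.
; MakePlan runs A*-style search over BP_GOAPNodes, scoring accumulated action cost plus unmet-goal count.
; It expands actions passing both state preconditions and CheckPrecondition on the owner's AIController, applying effects to child states.
; ReconstructPlan follows parent links and reverses the actions; the closed list never prunes revisited states.
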(event `self.ReceiveBeginPlay`
  (set `self.AIController` (`AIBlueprintHelperLibrary.GetAIController` (`self.GetOwner`))))

(fn `ApplyEffects`
  (params (OriginalState :type "Map of /Game/Dissertation/GOAP/E_WorldStates Enum to Boolean") (Effects :type "Map of /Game/Dissertation/GOAP/E_WorldStates Enum to Boolean"))
  (returns (NewState :type "Map of /Game/Dissertation/GOAP/E_WorldStates Enum to Boolean"))
  (locals (NState :type "Map of /Game/Dissertation/GOAP/E_WorldStates Enum to Boolean"))
  ;[0 0.1356 0.15 0.5] Loops through the Effects and adds them all to the original state, then returns the new state with effects applied
  (set `local.NState` OriginalState)
  (bind _keys (`BlueprintMapLibrary.Map_Keys` Effects))
  (for _array_element _keys
    ;;[0.15 0.04296 0.034 0.5] Bonus info, if there is already the same key it will just overwrite the value, Not create a new key/value
    (`BlueprintMapLibrary.Map_Add` (`local.NState`) _array_element (`BlueprintMapLibrary.Map_Find` Effects _array_element)))
  (return (`local.NState`)))

(fn `CalculateHeuristic`
  (params (CurrentState :type "Map of /Game/Dissertation/GOAP/E_WorldStates Enum to Boolean") (GoalState :type "Map of /Game/Dissertation/GOAP/E_WorldStates Enum to Boolean"))
  (returns (HeuristicCost :type "Float (double-precision)"))
  (locals (CostSoFar :type "Float (double-precision)"))
  ;[0 0.1356 0.15 0.5] Checks to see if the current state and goal state's keys have the same value(closer to the goal), if they are Not Equal then increment the Float(HeuristicCost)
  (bind _keys (`BlueprintMapLibrary.Map_Keys` GoalState))
  (for _array_element _keys
    (if (not (== (`BlueprintMapLibrary.Map_Find` CurrentState _array_element) (`BlueprintMapLibrary.Map_Find` GoalState _array_element)))
      (`/Engine/EditorBlueprintResources/StandardMacros.IncrementFloat` (`local.CostSoFar`))))
  ;[0 0.1356 0.15 0.5] Once Finished Return the Cost
  (return (`local.CostSoFar`)))

(fn `CheckCurrentWorldState`
  (params (CurrentState :type "Map of /Game/Dissertation/GOAP/E_WorldStates Enum to Boolean") (Requirments :type "Map of /Game/Dissertation/GOAP/E_WorldStates Enum to Boolean"))
  (returns (Success :type Boolean))
  ; Checks if the requirments are met by the current world state.
  (bind _keys (`BlueprintMapLibrary.Map_Keys` Requirments))
  (for _array_element _keys
    (bind (_value _returnvalue) (`BlueprintMapLibrary.Map_Find` CurrentState _array_element))
    ;;[0 0.1396 0.15 0.5] Checks if the Requirement is within the current state map.
    (if _returnvalue
      ;;[0 0.1356 0.15 0.5] Now it checks if the values of the maps are true(both the bools are true)
      (if (not (== _value (`BlueprintMapLibrary.Map_Find` Requirments _array_element)))
        (return false))
      (else
        (return false))))
  ;[0 0.1356 0.15 0.5] If the loop completes, it means that the current state and requirements match.
  (return true))

(fn `MakePlan`
  (params (CurrentWorldState :type "Map of /Game/Dissertation/GOAP/E_WorldStates Enum to Boolean") (GoalWorldState :type "Map of /Game/Dissertation/GOAP/E_WorldStates Enum to Boolean") (AvailableActions :type "Array of /Game/Dissertation/GOAP/Actions/BP_BaseActions Object Reference"))
  (returns (ThePlan :type "Array of /Game/Dissertation/GOAP/Actions/BP_BaseActions Object Reference") (Success :type Boolean))
  (locals (OpenList :type "Array of /Game/Dissertation/GOAP/BP_GOAPNode Object Reference") (ClosedList :type "Array of /Game/Dissertation/GOAP/BP_GOAPNode Object Reference") (CurrentProcessingNode :type "/Game/Dissertation/GOAP/BP_GOAPNode Object Reference") (LowestScore :type "Float (double-precision)" :default 999999.0) (BestNode :type "/Game/Dissertation/GOAP/BP_GOAPNode Object Reference") (CurrentState :type "Map of /Game/Dissertation/GOAP/E_WorldStates Enum to Boolean") (GoalState :type "Map of /Game/Dissertation/GOAP/E_WorldStates Enum to Boolean") (Actions :type "Array of /Game/Dissertation/GOAP/Actions/BP_BaseActions Object Reference") (ChildNode :type "/Game/Dissertation/GOAP/BP_GOAPNode Object Reference") (TempAction :type "/Game/Dissertation/GOAP/Actions/BP_BaseActions Object Reference"))
  (bind _currentprocessingnode (`local.CurrentProcessingNode`))
  (bind _openlist (`local.OpenList`))
  (bind _childnode (`local.ChildNode`))
  (bind _childnode_2 (`local.ChildNode`))
  (bind _openlist_2 (`local.OpenList`))
  (bind _bestnode (`local.BestNode`))
  (set `local.CurrentState` CurrentWorldState)
  (set `local.GoalState` GoalWorldState)
  (set `local.Actions` AvailableActions)
  ;[0 0.1356 0.15 0.5] This is the starting Node, it sets the all the relevant information passed in and then addes the node to the open list. This node will be the initial node used to check the Fullcost.
  (bind _returnvalue (`|GenericCreateObject` self "/Game/Dissertation/GOAP/BP_GOAPNode.BP_GOAPNode_C"))
  (set `local.CurrentProcessingNode` _returnvalue)
  (set `/Game/Dissertation/GOAP/BP_GOAPNode.WorldState` (`local.CurrentState`) _currentprocessingnode)
  (bind _output_get (set `/Game/Dissertation/GOAP/BP_GOAPNode.GivenCost` 0.0 _currentprocessingnode))
  (bind _heuristiccost (`self.CalculateHeuristic` (`local.CurrentState`) (`local.GoalState`)))
  (bind _output_get_2 (set `/Game/Dissertation/GOAP/BP_GOAPNode.HeuristicCost` _heuristiccost _currentprocessingnode))
  (set `/Game/Dissertation/GOAP/BP_GOAPNode.FullCost` (+ _output_get_2 _output_get) _currentprocessingnode)
  (`KismetArrayLibrary.Array_Add` _openlist (`local.CurrentProcessingNode`))
  ;[0 0.1356 0.15 0.5] This goes through every item in the openlist and checks to see which has the lowest Full cost, The firts node will is a bit overkill as there is only one node in there but it will be more relevant Later. It then sets the best node out of the bunch.
  (while (> (`KismetArrayLibrary.Array_Length` _openlist) 0)
    (set `local.LowestScore` 999999.0)
    (for _array_element _openlist_2
      (bind _fullcost (`/Game/Dissertation/GOAP/BP_GOAPNode.FullCost` _array_element))
      (if (< _fullcost (`local.LowestScore`))
        (set `local.LowestScore` _fullcost)
        (set `local.BestNode` _array_element)))
    ;[0 0.1356 0.15 0.5] This checks to see f the best node matches the current world state.
    (`KismetArrayLibrary.Array_RemoveItem` _openlist_2 _bestnode)
    (`KismetArrayLibrary.Array_Add` (`local.ClosedList`) _bestnode)
    (bind _success (`self.CheckCurrentWorldState` (`/Game/Dissertation/GOAP/BP_GOAPNode.WorldState` _bestnode) (`local.GoalState`)))
    (if _success
      ;[0 0.1356 0.15 0.5] If a plan has been found reverses it and passes in the new plan.
      (bind _theplan (`self.ReconstructPlan` (`local.BestNode`)))
      (return _theplan true)
      (else
        (for _array_element_2 (`local.Actions`)
          (set `local.TempAction` _array_element_2)
          (bind _success_2 (`self.CheckCurrentWorldState` (`/Game/Dissertation/GOAP/BP_GOAPNode.WorldState` (`local.BestNode`)) (`/Game/Dissertation/GOAP/Actions/BP_BaseActions.Preconditions` _array_element_2)))
          (if _success_2
            (bind _success_3 (`/Game/Dissertation/GOAP/Actions/BP_BaseActions.CheckPrecondition` (`local.TempAction`) (`self.AIController`)))
            (if _success_3
              (bind _returnvalue_2 (`|GenericCreateObject` self "/Game/Dissertation/GOAP/BP_GOAPNode.BP_GOAPNode_C"))
              (bind _output_get_3 (set `local.ChildNode` _returnvalue_2))
              (set `/Game/Dissertation/GOAP/BP_GOAPNode.ParentNode` (`local.BestNode`) _output_get_3)
              (set `/Game/Dissertation/GOAP/BP_GOAPNode.Action` (`local.TempAction`) (`local.ChildNode`))
              (bind _newstate (`self.ApplyEffects` self (`/Game/Dissertation/GOAP/BP_GOAPNode.WorldState` (`local.BestNode`)) (`/Game/Dissertation/GOAP/Actions/BP_BaseActions.Effects` (`local.TempAction`))))
              (set `/Game/Dissertation/GOAP/BP_GOAPNode.WorldState` _newstate _childnode)
              (set `/Game/Dissertation/GOAP/BP_GOAPNode.GivenCost` (+ (`/Game/Dissertation/GOAP/BP_GOAPNode.GivenCost` (`local.BestNode`)) (`/Game/Dissertation/GOAP/Actions/BP_BaseActions.Cost` (`local.TempAction`))) _childnode)
              (bind _heuristiccost_2 (`self.CalculateHeuristic` (`/Game/Dissertation/GOAP/BP_GOAPNode.WorldState` _childnode) (`local.GoalState`)))
              (bind _output_get_4 (set `/Game/Dissertation/GOAP/BP_GOAPNode.HeuristicCost` _heuristiccost_2 _childnode_2))
              (set `/Game/Dissertation/GOAP/BP_GOAPNode.FullCost` (+ _output_get_4 (`/Game/Dissertation/GOAP/BP_GOAPNode.GivenCost` _childnode_2)) _childnode_2)
              (`KismetArrayLibrary.Array_Add` (`local.OpenList`) (`local.ChildNode`)))))))))

(fn `ReconstructPlan`
  (params (BestNode :type "/Game/Dissertation/GOAP/BP_GOAPNode Object Reference"))
  (returns (ThePlan :type "Array of /Game/Dissertation/GOAP/Actions/BP_BaseActions Object Reference"))
  (locals (CurrentNode :type "/Game/Dissertation/GOAP/BP_GOAPNode Object Reference") (ActionList :type "Array of /Game/Dissertation/GOAP/Actions/BP_BaseActions Object Reference"))
  (bind _currentnode (`local.CurrentNode`))
  (bind _actionlist (`local.ActionList`))
  ;[0 0.1356 0.15 0.5] The way the nodes are set they are all children of eachother, so this checks if the current node is parented to anything, when its not it has found the start node, and the full plan.
  (set `local.CurrentNode` BestNode)
  (while (`KismetSystemLibrary.IsValid` (`/Game/Dissertation/GOAP/BP_GOAPNode.ParentNode` (`local.CurrentNode`)))
    ;[0 0.1356 0.15 0.5] Takes the Current nodes actions and adds it to an action list
    (`KismetArrayLibrary.Array_Add` (`local.ActionList`) (`/Game/Dissertation/GOAP/BP_GOAPNode.Action` _currentnode))
    (set `local.CurrentNode` (`/Game/Dissertation/GOAP/BP_GOAPNode.ParentNode` _currentnode)))
  ;[0 0.1356 0.15 0.5] Reverse the plan to put it in the correct order and returns it
  (`KismetArrayLibrary.Array_Reverse` _actionlist)
  (return _actionlist))