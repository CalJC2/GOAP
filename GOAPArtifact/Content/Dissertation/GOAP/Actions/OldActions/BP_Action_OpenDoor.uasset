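; GOAP action Blueprint that lets an AI agent open its target door.
; The precondition passes only when the AI controller's TargetDoor is valid and not locked.
; Start calls OpenCloseDoor on that door, and ActionExecuted immediately returns a fixed status enum value.
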(fn `ActionExecuted`
  (params (AiController :type "/Game/Dissertation/AI_NPC/BP_AIController Object Reference") (DeltaTime :type "Float (double-precision)"))
  (returns (ActionState :type "/Game/Dissertation/GOAP/E_ActionState Enum"))
  (return "NewEnumerator1"))

(fn `CheckPrecondition`
  (params (AIController :type "/Game/Dissertation/AI_NPC/BP_AIController Object Reference"))
  (returns (Success :type Boolean))
  ; Checks if the door is close and if its locked
  (bind _asbp_aicontroller (cast `/Game/Dissertation/AI_NPC/BP_AIController` AIController))
  (bind _targetdoor (`/Game/Dissertation/AI_NPC/BP_AIController.TargetDoor` _asbp_aicontroller))
  (if (`KismetSystemLibrary.IsValid` _targetdoor)
    (if (`/Game/Dissertation/LevelContent/BP_Door.IsLocked` _targetdoor)
      (return false)
      (else
        (return true)))
    (else
      (return false))))

(fn `Start`
  (params (AIController :type "/Game/Dissertation/AI_NPC/BP_AIController Object Reference"))
  (`/Game/Dissertation/LevelContent/I_Interactable.OpenCloseDoor` (`/Game/Dissertation/AI_NPC/BP_AIController.TargetDoor` AIController)))