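; GOAP action Blueprint that lets an AI-controlled NPC pick up a stamina object.
; Its precondition passes when the NPC is within a fixed distance of the controller's target stamina object.
; Start adds a fixed amount to the NPC's stamina and destroys that object immediately, with no clamp or validity check.
; ActionExecuted does no per-tick work and returns a constant status enum value.
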(fn `ActionExecuted`
  (params (AiController :type "/Game/Dissertation/AI_NPC/BP_AIController Object Reference") (DeltaTime :type "Float (double-precision)"))
  (returns (ActionState :type "/Game/Dissertation/GOAP/E_ActionState Enum"))
  (return "NewEnumerator1"))

(fn `CheckPrecondition`
  (params (AIController :type "/Game/Dissertation/AI_NPC/BP_AIController Object Reference"))
  (returns (Success :type Boolean))
  (if (< (`KismetMathLibrary.Vector_Distance` (`SceneComponent.K2_GetComponentLocation` (`Actor.RootComponent` (`/Game/Dissertation/AI_NPC/BP_AIController.NPC` AIController))) (`SceneComponent.K2_GetComponentLocation` (`/Game/Dissertation/LevelContent/BP_StaminaObject.DefaultSceneRoot` (`/Game/Dissertation/AI_NPC/BP_AIController.TargetStaminaObject` AIController)))) 200.0)
    (return true)
    (else
      (return false))))

(fn `Start`
  (params (AIController :type "/Game/Dissertation/AI_NPC/BP_AIController Object Reference"))
  (bind _npc (`/Game/Dissertation/AI_NPC/BP_AIController.NPC` AIController))
  (set `/Game/Dissertation/AI_NPC/BP_NPC.Stamina` (+ (`/Game/Dissertation/AI_NPC/BP_NPC.Stamina` _npc) 25.0) _npc)
  (`Actor.K2_DestroyActor` (`/Game/Dissertation/AI_NPC/BP_AIController.TargetStaminaObject` AIController)))