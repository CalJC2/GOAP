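; GOAP action Blueprint, stored under OldActions, that walks an AI agent to its target door.
; The precondition passes when the BP_AIController holds a valid TargetDoor.
; Start issues a MoveToActor toward that door, and each execution maps the controller's idle, waiting or moving status to an action result enum.
; Idle is not checked against actual arrival at the door.
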(fn `ActionExecuted`
  (params (AiController :type "/Game/Dissertation/AI_NPC/BP_AIController Object Reference") (DeltaTime :type "Float (double-precision)"))
  (returns (ActionState :type "/Game/Dissertation/GOAP/E_ActionState Enum"))
  (switch `EPathFollowingStatus` (`AIController.GetMoveStatus` AiController)
    (:`Idle`
      (return "NewEnumerator1"))
    (:`Waiting`
      (return "NewEnumerator2"))
    (:`Moving`
      (return "NewEnumerator0"))))

(fn `CheckPrecondition`
  (params (AIController :type "/Game/Dissertation/AI_NPC/BP_AIController Object Reference"))
  (returns (Success :type Boolean))
  (bind _asbp_aicontroller (cast `/Game/Dissertation/AI_NPC/BP_AIController` AIController))
  (`/Game/Dissertation/AI_NPC/BP_AIController.TargetDoor` _asbp_aicontroller
    (:`then`
      (return true))
    (:`else`
      (return false))))

(fn `Start`
  (params (AIController :type "/Game/Dissertation/AI_NPC/BP_AIController Object Reference"))
  (`AIController.MoveToActor` AIController (`/Game/Dissertation/AI_NPC/BP_AIController.TargetDoor` AIController) -1.0 true true true null true))