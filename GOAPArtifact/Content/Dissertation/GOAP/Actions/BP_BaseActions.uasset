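; BP_BaseActions is the base GOAP action for AI controllers, with overridable Start, ActionExecuted and Stop hooks.
; CheckPrecondition passes only if every entry in the Preconditions map matches the controller's CurrentWorldState.
; By default, Start does nothing and ActionExecuted returns a fixed enum value, while Stop clears NeedsToStop and halts the controller's movement.
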(fn `ActionExecuted`
  (params (AiController :type "/Game/Dissertation/AI_NPC/GOAP/BP_AIControllerGOAP Object Reference") (DeltaTime :type "Float (double-precision)"))
  (returns (ActionState :type "/Game/Dissertation/GOAP/E_ActionState Enum"))
  (return "NewEnumerator0"))

(fn `CheckPrecondition`
  (params (AIController :type "/Game/Dissertation/AI_NPC/GOAP/BP_AIControllerGOAP Object Reference"))
  (returns (Success :type Boolean))
  (bind _keys (`BlueprintMapLibrary.Map_Keys` (`self.Preconditions`)))
  (for _array_element _keys
    (if (not (== (`BlueprintMapLibrary.Map_Find` (`self.Preconditions`) _array_element) (`BlueprintMapLibrary.Map_Find` (`/Game/Dissertation/AI_NPC/GOAP/BP_AIControllerGOAP.CurrentWorldState` AIController) _array_element)))
      (return false)))
  (return true))

(fn `Start`
  (params (AIController :type "/Game/Dissertation/AI_NPC/GOAP/BP_AIControllerGOAP Object Reference")))

(fn `Stop`
  (params (AIController :type "AIController Object Reference"))
  (set `self.NeedsToStop` false)
  (`Controller.StopMovement` AIController))