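; A GOAP action that sends an AI-controlled NPC to collect a stamina item.
; Start picks the nearest of the NPC's known stamina items and stores it as the controller's target.
; Execution issues a single move order, then polls move status; arriving within range destroys the item and refills stamina.
; Each poll returns an enum status, with stop requests, waiting, or idling out of range sharing one result.
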(fn `ActionExecuted`
  (params (AiController :type "/Game/Dissertation/AI_NPC/BP_AIController Object Reference") (DeltaTime :type "Float (double-precision)"))
  (returns (ActionState :type "/Game/Dissertation/GOAP/E_ActionState Enum"))
  (bind _targetstaminaobject (`/Game/Dissertation/AI_NPC/BP_AIController.TargetStaminaObject` AiController))
  (bind _targetstaminaobject_2 (`/Game/Dissertation/AI_NPC/BP_AIController.TargetStaminaObject` AiController))
  (bind _npc (`/Game/Dissertation/AI_NPC/BP_AIController.NPC` AiController))
  (bind _returnvalue (`SceneComponent.K2_GetComponentLocation` (`/Game/Dissertation/LevelContent/BP_StaminaObject.DefaultSceneRoot` _targetstaminaobject_2)))
  (if (`self.NeedsToStop`)
    (return "NewEnumerator2")
    (elif (`self.StartedMoving`)
      (switch `EPathFollowingStatus` (`AIController.GetMoveStatus` AiController)
        (:`Idle`
          (if (< (`Actor.GetDistanceTo` _targetstaminaobject _npc) 50.0)
            (`Actor.K2_DestroyActor` _targetstaminaobject)
            (set `/Game/Dissertation/AI_NPC/BP_NPC.Stamina` 100.0 _npc)
            (set `/Game/Dissertation/AI_NPC/BP_AIController.TargetStaminaObject` null AiController)
            (return "NewEnumerator1")
            (else
              (return "NewEnumerator2"))))
        (:`Waiting`
          (return "NewEnumerator2"))
        (:`Moving`
          (return "NewEnumerator0")))
      (else
        (`/Engine/EditorBlueprintResources/StandardMacros.IsValid` _targetstaminaobject_2
          (:`Is Valid`
            (`AIController.MoveToLocation` AiController _returnvalue -1.0 true true false true null true)
            (set `self.StartedMoving` true)
            (`KismetSystemLibrary.PrintString` null (`KismetStringLibrary.Conv_VectorToString` _returnvalue))))))))

(fn `Start`
  (params (AIController :type "/Game/Dissertation/AI_NPC/BP_AIController Object Reference"))
  (locals (ClosestDistance :type "Float (double-precision)"))
  (bind _npc (`/Game/Dissertation/AI_NPC/BP_AIController.NPC` AIController))
  (set `self.StartedMoving` false)
  (set `local.ClosestDistance` 99999999.0)
  (for _array_element (`/Game/Dissertation/AI_NPC/BP_NPC.KnownStaminaItems` _npc)
    (bind _returnvalue (`Actor.GetDistanceTo` _array_element _npc))
    (if (< _returnvalue (`local.ClosestDistance`))
      (set `local.ClosestDistance` _returnvalue)
      (set `/Game/Dissertation/AI_NPC/BP_AIController.TargetStaminaObject` _array_element AIController))))