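; GOAP search action that sends an NPC running to a random location.
; Start resets the wait timer and, if the AI controller finds a location, raises walk speed and issues the move.
; ActionExecuted polls move status, keeping one result while moving or briefly idle and switching once the idle wait elapses.
; A stop request or a Waiting move status returns a third result.
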(fn `ActionExecuted`
  (params (AiController :type "/Game/Dissertation/AI_NPC/GOAP/BP_AIControllerGOAP Object Reference") (DeltaTime :type "Float (double-precision)"))
  (returns (ActionState :type "/Game/Dissertation/GOAP/E_ActionState Enum"))
  (if (`self.NeedsToStop`)
    (return "NewEnumerator2")
    (else
      (switch `EPathFollowingStatus` (`AIController.GetMoveStatus` AiController)
        (:`Idle`
          (bind _output_get (set `self.CurrentWaitTime` (+ DeltaTime (`self.CurrentWaitTime`))))
          (if (>= _output_get 0.5)
            (return "NewEnumerator1")
            (else
              (return "NewEnumerator0"))))
        (:`Waiting`
          (return "NewEnumerator2"))
        (:`Moving`
          (return "NewEnumerator0"))))))

(fn `Start`
  (params (AIController :type "/Game/Dissertation/AI_NPC/GOAP/BP_AIControllerGOAP Object Reference"))
  (set `self.CurrentWaitTime` 0.0)
  (bind (_location _locationfound) (`/Game/Dissertation/AI_NPC/GOAP/BP_AIControllerGOAP.FindRandomLocation` AIController))
  (if _locationfound
    (set `CharacterMovementComponent.MaxWalkSpeed` 600.0 (`Character.CharacterMovement` (`/Game/Dissertation/AI_NPC/GOAP/BP_AIControllerGOAP.NPC` AIController)))
    (`AIController.MoveToLocation` AIController _location -1.0 true true false true null true)))