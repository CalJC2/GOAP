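; BP_Action_Hide is a GOAP action that sends an AI to a hiding spot, with a precondition that always passes.
; Start resets its movement flag and asks the AI controller to run an EQS query for a hiding spot.
; ActionExecuted polls that query, issues a move to the best spot once ready, then maps the controller's move status or a query failure to the action's result.
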(fn `ActionExecuted`
  (params (AiController :type "/Game/Dissertation/AI_NPC/BP_AIController Object Reference") (DeltaTime :type "Float (double-precision)"))
  (returns (ActionState :type "/Game/Dissertation/GOAP/E_ActionState Enum"))
  (if (`self.HasStarteMoving`)
    (switch `EPathFollowingStatus` (`AIController.GetMoveStatus` AiController)
      (:`Idle`
        (return "NewEnumerator1"))
      (:`Waiting`
        (return "NewEnumerator2"))
      (:`Moving`
        (return "NewEnumerator0")))
    (elif (`/Game/Dissertation/AI_NPC/BP_AIController.IsEQSReady` AiController)
      (`AIController.MoveToLocation` AiController (`/Game/Dissertation/AI_NPC/BP_AIController.BestHidingSpot` AiController) -1.0 true true false true null true)
      (set `self.HasStarteMoving` true)
      (return "NewEnumerator0")
      (elif (`/Game/Dissertation/AI_NPC/BP_AIController.IsEQSFailed` AiController)
        (return "NewEnumerator2")
        (else
          (return "NewEnumerator0"))))))

(fn `CheckPrecondition`
  (params (AIController :type "AIController Object Reference"))
  (returns (Success :type Boolean))
  (return true))

(fn `Start`
  (params (AIController :type "/Game/Dissertation/AI_NPC/BP_AIController Object Reference"))
  (set `self.HasStarteMoving` false)
  (`/Game/Dissertation/AI_NPC/BP_AIController.FindHidingSpotEQS` AIController))