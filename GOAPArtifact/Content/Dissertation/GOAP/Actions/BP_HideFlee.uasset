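; GOAP action that sends an NPC fleeing to a hiding spot.
; Start sets a faster walk speed and launches an EQS query through the AI controller to find the best spot.
; Each execution waits for the query, issues the move, then polls move status, returning an enum result for in-progress, arrival, or failure, including failed queries and stop requests.
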(fn `ActionExecuted`
  (params (AiController :type "/Game/Dissertation/AI_NPC/GOAP/BP_AIControllerGOAP Object Reference") (DeltaTime :type "Float (double-precision)"))
  (returns (ActionState :type "/Game/Dissertation/GOAP/E_ActionState Enum"))
  (if (`self.NeedsToStop`)
    (return "NewEnumerator2")
    (elif (`self.StartedMoving`)
      (switch `EPathFollowingStatus` (`AIController.GetMoveStatus` AiController)
        (:`Idle`
          (return "NewEnumerator1"))
        (:`Waiting`
          (return "NewEnumerator2"))
        (:`Moving`
          (return "NewEnumerator0")))
      (elif (`/Game/Dissertation/AI_NPC/GOAP/BP_AIControllerGOAP.HideEQSReady` AiController)
        (bind _returnvalue (`AIController.MoveToLocation` AiController (`/Game/Dissertation/AI_NPC/GOAP/BP_AIControllerGOAP.BestHidingSpot` AiController) -1.0 true true false true null true))
        (switch `EPathFollowingRequestResult` _returnvalue
          (:`Failed`
            (return "NewEnumerator2"))
          (:`AlreadyAtGoal`
            (return "NewEnumerator1"))
          (:`RequestSuccessful`
            (set `self.StartedMoving` true)
            (return "NewEnumerator0")))
        (elif (`/Game/Dissertation/AI_NPC/GOAP/BP_AIControllerGOAP.HideEQSFailed` AiController)
          (return "NewEnumerator2")
          (else
            (return "NewEnumerator0")))))))

(fn `Start`
  (params (AIController :type "/Game/Dissertation/AI_NPC/GOAP/BP_AIControllerGOAP Object Reference"))
  (locals (NewLocalVar :type "/Game/Dissertation/AI_NPC/GOAP/BP_AIControllerGOAP Object Reference"))
  (set `self.StartedMoving` false)
  (set `CharacterMovementComponent.MaxWalkSpeed` 600.0 (`Character.CharacterMovement` (`/Game/Dissertation/AI_NPC/GOAP/BP_AIControllerGOAP.NPC` AIController)))
  (`/Game/Dissertation/AI_NPC/GOAP/BP_AIControllerGOAP.FindHidingSpotEQS` AIController))