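; BP_Action_Search is a GOAP action that sends an AI to search by moving to a random patrol location.
; Start asks the AI controller for a random patrol location and issues a move only if one is found.
; ActionExecuted maps the controller's move status (idle, waiting or moving) to an action result enum.
; Its precondition check always passes.
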(fn `ActionExecuted`
  (params (AiController :type "/Game/Dissertation/AI_NPC/BP_AIController Object Reference") (DeltaTime :type "Float (double-precision)"))
  (returns (ActionState :type "/Game/Dissertation/GOAP/E_ActionState Enum"))
  (switch `EPathFollowingStatus` (`AIController.GetMoveStatus` AiController)
    (:`Idle`
      (return "NewEnumerator1"))
    (:`Waiting`
      (return "NewEnumerator2"))
    (:`Moving`
      (return "NewEnumerator0"))))

(fn `CheckPrecondition`
  (params (AIController :type "AIController Object Reference"))
  (returns (Success :type Boolean))
  (return true))

(fn `Start`
  (params (AIController :type "/Game/Dissertation/AI_NPC/BP_AIController Object Reference"))
  (bind (_location _locationfound) (`/Game/Dissertation/AI_NPC/BP_AIController.FindRandomPatrolLocation` AIController))
  (if _locationfound
    (`AIController.MoveToLocation` AIController _location -1.0 true true false true null true)))