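; BP_Door is a hinged door actor that toggles open and closed through OpenCloseDoor unless it is locked.
; BeginPlay stores the starting yaw as closed and a 90-degree offset from it as open.
; A timeline lerps the root component's world yaw between the two, playing forward to open and in reverse to close.
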(event `self.ReceiveBeginPlay`
  (bind (_returnvalue_roll _returnvalue_pitch _returnvalue_yaw) (`KismetMathLibrary.BreakRotator` (`SceneComponent.K2_GetComponentRotation` (`self.DefaultSceneRoot`))))
  (bind _output_get (set `self.DoorClosePosition` _returnvalue_yaw))
  (set `self.DoorOpenPosition` (+ _output_get 90.0)))

(event `OpenDoor`
  (set `self.IsDoorOpen` true)
  (bind (_direction _dooropentrack) (`Timeline|DoorOpen/Close` :!label _label)
    (:`Update`
      (`SceneComponent.K2_SetWorldRotation` (`self.DefaultSceneRoot`) (`KismetMathLibrary.MakeRotator` 0.0 0.0 (`KismetMathLibrary.Lerp` (`self.DoorClosePosition`) (`self.DoorOpenPosition`) _dooropentrack)) false false))))

(event `CloseDoor`
  (set `self.IsDoorOpen` false)
  (goto _label :!via `Reverse`))

(event `/Game/Dissertation/LevelContent/I_Interactable.OpenCloseDoor`
  (if (`self.IsLocked`)
    _
    (elif (`self.IsDoorOpen`)
      (`self.CloseDoor`)
      (else
        (`self.OpenDoor`)))))

(fn `UserConstructionScript`)