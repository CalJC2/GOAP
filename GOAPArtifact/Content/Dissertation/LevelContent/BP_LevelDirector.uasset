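; Level director for a first-person dissertation playtest level, logging catch data and shuffling doors during play.
; BeginPlay clears a hard-coded save file, toggles every door and starts two looping timers.
; Each AI catch appends the HUD timer and caught count to that file.
; ChangeDoor toggles the current door and a random replacement; SpawnStamina is empty, with its random spawn-point logic left disconnected.
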(event `self.ReceiveBeginPlay`
  (bind _doorarray (`self.DoorArray`))
  (bind _asbp_first_person_character (cast `/Game/FirstPerson/Blueprints/BP_FirstPersonCharacter` (`GameplayStatics.GetPlayerCharacter` 0)))
  (bind _output_get (set `self.Player` _asbp_first_person_character))
  (`FileSDKBPLibrary.CreateFile` "C:\\Users\\user\\OneDrive - UWE Bristol\\Documents\\Calum\\Year3\\CCTP\\SavedData\\P1_B")
  (add `self.AICaught` (delegate `OnAICaught`))
  (set `self.MaxStaminaArrayValue` (`KismetArrayLibrary.Array_Length` (`self.StaminaSpawnPointsArray`)))
  (set `self.MaxDoorArrayValue` (`KismetArrayLibrary.Array_Length` _doorarray))
  (for _array_element _doorarray
    (message `/Game/Dissertation/LevelContent/I_Interactable.OpenCloseDoor` _array_element))
  (`KismetSystemLibrary.K2_SetTimerDelegate` (`|CreateDelegate` :!event `Spawn Stamina`) 5.0 true true 1.0 1.0)
  (`KismetSystemLibrary.K2_SetTimerDelegate` (`|CreateDelegate` :!event `ChangeDoor`) 15.0 true true 5.0))

(event `OnAICaught`
  (bind _hudwidget (`/Game/FirstPerson/Blueprints/BP_FirstPersonCharacter.HUDWidget` (stale `self.ReceiveBeginPlay` _output_get)))
  (`FileSDKBPLibrary.WriteStringToFile` "C:\\Users\\user\\OneDrive - UWE Bristol\\Documents\\Calum\\Year3\\CCTP\\SavedData\\P1_B" (`KismetStringLibrary.Concat_StrStr` (`KismetSystemLibrary.MakeLiteralString` (`KismetStringLibrary.Conv_DoubleToString` (`/Game/Dissertation/UI/WBP_HUD.TimerFloat` _hudwidget))) ": " (`KismetSystemLibrary.MakeLiteralString` (`KismetStringLibrary.Conv_IntToString` (`/Game/Dissertation/UI/WBP_HUD.CaughtInt` _hudwidget))) "\\n ") true))

(event `self.ReceiveTick`
  (params (DeltaSeconds :type "Float (single-precision)")))

(event `ChangeDoor`
  (bind _output (`|GetArrayItem` (`self.DoorArray`) (`KismetMathLibrary.RandomIntegerInRange` 0 (`self.MaxDoorArrayValue`))))
  (if (== (`self.CurrentDoor`) _output)
    (`self.ChangeDoor`)
    (else
      (message `/Game/Dissertation/LevelContent/I_Interactable.OpenCloseDoor` (`self.CurrentDoor`))
      (bind _output_get (set `self.CurrentDoor` _output))
      (message `/Game/Dissertation/LevelContent/I_Interactable.OpenCloseDoor` _output_get))))

(event `Spawn Stamina`)

(fn `UserConstructionScript`)