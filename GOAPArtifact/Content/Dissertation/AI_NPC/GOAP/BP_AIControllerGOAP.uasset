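; GOAP AI controller for an NPC that evades the player, restores low stamina or otherwise falls back to a default goal.
; Action objects are instanced at BeginPlay, and each Tick rebuilds a boolean world state from stamina, sight, distance, doors and a camera-to-socket hidden trace.
; An Idle/Planning/Acting state machine gets plans from BPCPlanner and runs them stepwise, replanning on failure.
; EQS queries supply hiding and flee locations.
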(event Custom|StartStep
  (if (< (Variables|GOAP|GetCurrentStepIndex) (Utilities|Array|Length (Variables|GOAP|GetCurrentPlan)))
    (bind _output_get (Variables|GOAP|SetCurrentAction (Utilities|Array|Get(acopy) (Variables|GOAP|GetCurrentPlan) (Variables|GOAP|GetCurrentStepIndex))))
    (Development|PrintString (Utilities|GetDisplayName _output_get))
    (Default|Start _output_get self)
    (else
      (Variables|GOAP|SetPlanningState "NewEnumerator0"))))

(event Custom|FindHidingSpotEQS
  (Variables|Hide|SetHideEQSReady false)
  (Variables|Hide|SetHideEQSFailed false)
  (bind _returnvalue (AI|EQS|RunEQSQuery "/Game/Dissertation/AI_NPC/EQS/EQS_FindHidingSpot.EQS_FindHidingSpot" self "RandomBest5Pct"))
  (EventDispatchers|AssignOnQueryFinishedEvent _returnvalue (delegate Custom|OnHidingFinishedEvent)))

(event Custom|RunFleeEQS
  (Variables|Flee|SetFleeEQSReady false)
  (Variables|Flee|SetFleeEQSFailed false)
  (bind _returnvalue (AI|EQS|RunEQSQuery "/Game/Dissertation/AI_NPC/EQS/EQS_FindFleeSpot.EQS_FindFleeSpot" self "RandomBest5Pct"))
  (EventDispatchers|AssignOnQueryFinishedEvent _returnvalue (delegate Custom|OnFleeFinishedEvent)))

(event Custom|StaminaCheck
  (bind _npc (Variables|GOAP|GetNPC))
  (bind _capsulecomponent (Variables|/Script/Engine.Character|GetCapsuleComponent _npc))
  (bind _returnvalue (Transformation|GetWorldLocation _capsulecomponent))
  (bind _outhit (Collision|SphereTraceByChannel _returnvalue _returnvalue 5e+01 "TraceTypeQuery1" false 0 "None"))
  (if (Class|GameplayStatics|ObjectIsA (.HitActor (Collision|BreakHitResult _outhit)) "/Game/Dissertation/LevelContent/BP_StaminaObject.BP_StaminaObject_C")
    (Actor|DestroyActor (.HitActor (Collision|BreakHitResult _outhit)))
    (Variables|/Game/Dissertation/AI_NPC/GOAP/BP_NPCGOAP.BP_NPCGOAP_C|SetStamina (Variables|GOAP|GetNPC) 1e+02)))

(event Custom|OnFleeFinishedEvent
  (params (QueryInstance :type Env%20Query%20Instance%20Blueprint%20Wrapper%20Object%20Reference) (QueryStatus :type EEnvQueryStatus%20Enum :default "Processing"))
  (bind _resultlocations (AI|EQS|GetQueryResultsasLocations QueryInstance))
  (if (> (Utilities|Array|Length _resultlocations) 0)
    (Variables|Flee|SetBestFleeLocation (Utilities|Array|Get(acopy) _resultlocations))
    (Variables|Flee|SetFleeEQSReady true)
    (else
      (Variables|Flee|SetFleeEQSFailed true))))

(event Custom|OnHidingFinishedEvent
  (params (QueryInstance :type Env%20Query%20Instance%20Blueprint%20Wrapper%20Object%20Reference) (QueryStatus :type EEnvQueryStatus%20Enum :default "Processing"))
  (bind _resultlocations (AI|EQS|GetQueryResultsasLocations QueryInstance))
  (if (> (Utilities|Array|Length _resultlocations) 0)
    (Variables|Hide|SetBestHidingSpot (Utilities|Array|Get(acopy) _resultlocations))
    (Variables|Hide|SetHideEQSReady true)
    (else
      (Variables|Hide|SetHideEQSFailed true))))

(event EventTick
  (params (DeltaSeconds :type Float%20%28single-precision%29))
  (bind _self self)
  (Variables|Default|SetDeltaTime DeltaSeconds)
  (CallFunction|UpdateWorldState)
  (switch Utilities|FlowControl|Switch|SwitchonE_PlannerState (Variables|GOAP|GetPlanningState)
    (:NewEnumerator0
      (Utilities|Array|Clear (Variables|GOAP|GetCurrentPlan))
      (Variables|GOAP|SetCurrentAction 0)
      ;[0 0.1356 0.15 0.5] No plan, Reset to planning
      (Utilities|FlowControl|Delay 0.2)
      (Variables|GOAP|SetPlanningState "NewEnumerator1"))
    (:NewEnumerator1
      ;[0 0.1356 0.15 0.5] Sets the Goal States, If player is close then Run, if the AI is low on Stamina then find stamina, else go idle(Patrol)
      (if (not (.Value (Utilities|Map|Find (Variables|GOAP|GetCurrentWorldState) "NewEnumerator9")))
        ;[0 0.1356 0.15 0.5] If the AI knows where the player is, Sets the Goal state and makes a plan for it!
        (bind (_theplan _success) (Default|MakePlan (Variables|Default|GetBPC_Planner) (Variables|GOAP|GetCurrentWorldState) (Utilities|Map|MakeMap "NewEnumerator9" true) (Variables|GOAP|GetAvailableActions)))
        (if _success
          (Variables|GOAP|SetCurrentPlan _theplan)
          ;[0 0.1356 0.15 0.5] If there is a plan, Act
          (Variables|GOAP|SetCurrentStepIndex 0 :!label _label)
          (Variables|GOAP|SetPlanningState "NewEnumerator2")
          (CallFunction|StartStep)
          (else
            ;[0 0.1356 0.15 0.5] If there isnt a plan, Idle
            (Variables|GOAP|SetPlanningState "NewEnumerator0" :!label _label_2)))
        (elif (.Value (Utilities|Map|Find (Variables|GOAP|GetCurrentWorldState) "NewEnumerator11"))
          ;[0 0.1356 0.15 0.5] If the AI is running low on stamina, Sets the GoalState and makes a plan for it
          (bind (_theplan_2 _success_2) (Default|MakePlan (Variables|Default|GetBPC_Planner) (Variables|GOAP|GetCurrentWorldState) (Utilities|Map|MakeMap "NewEnumerator12" true) (Variables|GOAP|GetAvailableActions)))
          (if _success_2
            (Variables|GOAP|SetCurrentPlan _theplan_2)
            (goto _label)
            (else
              (goto _label_2)))
          (else
            (bind (_theplan_3 _success_3) (Default|MakePlan (Variables|Default|GetBPC_Planner) (Variables|GOAP|GetCurrentWorldState) (Utilities|Map|MakeMap "NewEnumerator17" true) (Variables|GOAP|GetAvailableActions)))
            (if _success_3
              (Variables|GOAP|SetCurrentPlan _theplan_3)
              (goto _label)
              (else
                (goto _label_2)))))))
    (:NewEnumerator2
      (bind _currentaction (Variables|GOAP|GetCurrentAction)
        (:then
          (bind _success_4 (Default|CheckPrecondition _currentaction _self))
          (if _success_4
            (bind _actionstate (Default|ActionExecuted (Variables|GOAP|GetCurrentAction) self (Variables|Default|GetDeltaTime)))
            (switch Utilities|FlowControl|Switch|SwitchonE_ActionState _actionstate
              (:NewEnumerator1
                (Math|Integer|IncrementInt (Variables|GOAP|GetCurrentStepIndex)
                  (:%20%20
                    (CallFunction|StartStep))))
              (:NewEnumerator2
                (Default|Stop (Variables|GOAP|GetCurrentAction) self)
                (Variables|GOAP|SetPlanningState "NewEnumerator0")))
            (else
              (Default|Stop (Variables|GOAP|GetCurrentAction) self)
              (Variables|GOAP|SetPlanningState "NewEnumerator0"))))
        (:else
          (Default|Stop _currentaction _self)
          (Variables|GOAP|SetPlanningState "NewEnumerator0"))))))

(event EventBeginPlay
  (bind _asbp_npcgoap (Utilities|Casting|CastToBP_NPCGOAP (Pawn|GetControlledPawn)))
  (Utilities|IsValid _asbp_npcgoap
    (:Is%20Valid
      (Variables|GOAP|SetNPC _asbp_npcgoap)
      (bind _asbp_first_person_character (Utilities|Casting|CastToBP_FirstPersonCharacter (Game|GetPlayerCharacter 0)))
      (Utilities|IsValid _asbp_first_person_character
        (:Is%20Valid
          (Variables|Default|SetPlayer _asbp_first_person_character)
          ;[0 0.1356 0.15 0.5] Setting all actions that can be used by this ai within the controller
          (for _array_element (Variables|GOAP|GetActionClasses)
            (bind _returnvalue (Game|ConstructObjectfromClass self _array_element (.ActionName (Utilities|GetClassDefaults _array_element)) (.Cost (Utilities|GetClassDefaults _array_element)) (.Preconditions (Utilities|GetClassDefaults _array_element)) (.Effects (Utilities|GetClassDefaults _array_element))))
            (Utilities|Array|Add (Variables|GOAP|GetAvailableActions) _returnvalue))
          (bind _outactors (Actor|GetAllActorsOfClass "/Game/Dissertation/LevelContent/BP_Door.BP_Door_C"))
          (for _array_element_2 _outactors
            (Utilities|Array|Add (Variables|Default|GetAllDoorsArray) _array_element_2)))))))

(fn ConstructionScript)

(fn UpdateWorldState
  (bind _updatestate (LocalVariables|GetUpdateState))
  (bind _updatestate_2 (LocalVariables|GetUpdateState))
  (bind _npc (Variables|GOAP|GetNPC))
  (bind _updatestate_3 (LocalVariables|GetUpdateState))
  (bind _updatestate_4 (LocalVariables|GetUpdateState))
  (bind _updatestate_5 (LocalVariables|GetUpdateState))
  (bind _updatestate_6 (LocalVariables|GetUpdateState))
  (bind _knownstaminaitems (Variables|/Game/Dissertation/AI_NPC/GOAP/BP_NPCGOAP.BP_NPCGOAP_C|GetKnownStaminaItems _npc))
  (Utilities|FlowControl|Sequence
    (:then_0
      (if (<= (Variables|/Game/Dissertation/AI_NPC/GOAP/BP_NPCGOAP.BP_NPCGOAP_C|GetStamina (Variables|GOAP|GetNPC)) 3e+01)
        (Utilities|Map|Add _updatestate_6 "NewEnumerator11" true)
        (else
          (Utilities|Map|Add _updatestate_6 "NewEnumerator11" false))))
    (:then_1
      (if (>= (Variables|/Game/Dissertation/AI_NPC/GOAP/BP_NPCGOAP.BP_NPCGOAP_C|GetStamina (Variables|GOAP|GetNPC)) 85.0)
        (Utilities|Map|Add _updatestate_5 "NewEnumerator12" true)
        (else
          (Utilities|Map|Add _updatestate_5 "NewEnumerator12" false))))
    (:then_2
      (bind _ishidden (CallFunction|CheckIsHidden))
      (Utilities|Map|Add (LocalVariables|GetUpdateState) "NewEnumerator13" _ishidden))
    (:then_3
      (bind _array_element (Utilities|Array|ForEachLoopwithBreak (Variables|Default|GetAllDoorsArray) :!label _label)
        (:LoopBody
          (if (<= (Transformation|GetDistanceTo (Variables|GOAP|GetNPC) _array_element) 2e+02)
            (bind _asbp_door (Utilities|Casting|CastToBP_Door _array_element))
            (if (Variables|/Game/Dissertation/LevelContent/BP_Door.BP_Door_C|GetIsDoorOpen _asbp_door)
              (Utilities|Map|Add (LocalVariables|GetUpdateState) "NewEnumerator14" true)
              (goto _label Break))))
        (:Completed
          (Utilities|Map|Add (LocalVariables|GetUpdateState) "NewEnumerator14" false))))
    (:then_4
      (if (Variables|/Game/Dissertation/AI_NPC/GOAP/BP_NPCGOAP.BP_NPCGOAP_C|GetCanSeePlayer (Variables|GOAP|GetNPC))
        (Utilities|Map|Add _updatestate_2 "NewEnumerator10" true)
        (else
          (Utilities|Map|Add _updatestate_2 "NewEnumerator10" false))))
    (:then_5
      (if (or (Variables|/Game/Dissertation/AI_NPC/GOAP/BP_NPCGOAP.BP_NPCGOAP_C|GetCanSeePlayer (Variables|GOAP|GetNPC)) (<= (Math|Vector|Distance(Vector) (Transformation|GetWorldLocation (Variables|/Script/Engine.Character|GetCapsuleComponent (Variables|GOAP|GetNPC))) (Transformation|GetWorldLocation (Variables|/Script/Engine.Character|GetCapsuleComponent (Variables|Default|GetPlayer)))) 5e+02))
        (Utilities|Map|Add _updatestate_3 "NewEnumerator9" false)
        (else
          (Utilities|Map|Add _updatestate_3 "NewEnumerator9" true))))
    (:then_6
      (for _array_element_2 _knownstaminaitems
        (Utilities|IsValid _array_element_2
          (:Is%20Not%20Valid
            (Utilities|Array|RemoveItem _knownstaminaitems _array_element_2))))
      (if (> (Utilities|Array|Length _knownstaminaitems) 0)
        (Utilities|Map|Add _updatestate "NewEnumerator16" true)
        (else
          (Utilities|Map|Add _updatestate "NewEnumerator16" false))))
    (:then_7
      (Utilities|Map|Add (LocalVariables|GetUpdateState) "NewEnumerator17" false))
    (:then_8
      (if (< (Transformation|GetDistanceTo (Variables|GOAP|GetNPC) (Variables|Default|GetPlayer)) 5e+02)
        (Utilities|Map|Add _updatestate_4 "NewEnumerator18" true)
        (else
          (Utilities|Map|Add _updatestate_4 "NewEnumerator18" false))))
    (:then_9
      (Variables|GOAP|SetCurrentWorldState (LocalVariables|GetUpdateState)))))

(fn FindRandomLocation
  (bind _returnvalue (Pawn|GetControlledPawn))
  (bind _returnvalue_2 (Transformation|GetActorLocation _returnvalue))
  (bind (_randomlocation _returnvalue_3) (AI|Navigation|GetRandomReachablePointinRadius _returnvalue_2 5e+03 0 0))
  (return _randomlocation _returnvalue_3))

(fn CheckIsHidden
  (for _array_element (LocalVariables|GetSocketsToCheck_0)
    (bind _outhit (Collision|LineTraceByChannel (Transformation|GetWorldLocation (Variables|/Script/GOAPArtifact.GOAPArtifactCharacter|GetFirstPersonCameraComponent (Variables|Default|GetPlayer))) (Transformation|GetSocketLocation (Variables|/Script/Engine.Character|GetMesh (Variables|GOAP|GetNPC)) _array_element) "TraceTypeQuery1" false (Utilities|Array|MakeArray (Game|Player|GetPlayerPawn 0)) "None" false))
    (if (Class|GameplayStatics|ObjectIsA (.hitactor _outhit) "/Game/Dissertation/AI_NPC/GOAP/BP_NPCGOAP.BP_NPCGOAP_C")
      (return false)
      (else
        (return true))))
  (return true))