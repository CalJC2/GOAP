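; BP_NPCBT is an AI NPC, likely driven by a Behavior Tree, that tracks player awareness, stamina and known stamina items.
; AI Perception updates set CanSeePlayer purely by the updated actor's class, without checking sensing success, and add stamina objects to a unique known-items list.
; Tick drains Stamina, cycles a one-second timer and counts time since seeing the player, a paranoia delay against turning back immediately after fleeing.
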(event `self.ReceiveTick`
  (params (DeltaSeconds :type "Float (single-precision)"))
  ; Parranoia condition, used in update world state so the NPC doesnt immediatley turn ito the player after fleeing
  (if (`self.CanSeePlayer`)
    (set `self.TimeSinceSawPlayer` 0.0))
  (set `self.TimeSinceSawPlayer` (+ (`self.TimeSinceSawPlayer`) DeltaSeconds))
  (set `self.Stamina` (- (`self.Stamina`) DeltaSeconds))
  (bind _output_get (set `self.Timer` (+ DeltaSeconds (`self.Timer`))))
  (if (> _output_get 1.0)
    (set `self.Timer` 0.0)))

(event `self.AIPerception.OnTargetPerceptionUpdated`
  (params (Actor :type "Actor Object Reference") (Stimulus :type "AIStimulus Structure"))
  ;[0 0.1356 0.15 0.5] If a Sense(currently sight, need to add Report Noise event node to player with a Pawn Noise Emitter component), it will set a bool
  (if (`GameplayStatics.ObjectIsA` Actor "/Game/FirstPerson/Blueprints/BP_FirstPersonCharacter.BP_FirstPersonCharacter_C")
    (set `self.CanSeePlayer` true)
    (else
      (set `self.CanSeePlayer` false)))
  (if (`GameplayStatics.ObjectIsA` Actor "/Game/Dissertation/LevelContent/BP_StaminaObject.BP_StaminaObject_C")
    (bind _asbp_stamina_object (cast `/Game/Dissertation/LevelContent/BP_StaminaObject` Actor))
    (`KismetArrayLibrary.Array_AddUnique` (`self.KnownStaminaItems`) _asbp_stamina_object)))

(fn `UserConstructionScript`)