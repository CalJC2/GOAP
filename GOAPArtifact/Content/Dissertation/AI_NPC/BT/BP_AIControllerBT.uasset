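; AI controller for the behavior tree NPC, which starts BT_NPCBehaviour on possess and tracks the NPC's condition relative to the player.
; BeginPlay caches the controlled BP_NPCBT and the first-person player character.
; Every tick, UpdateBT converts stamina thresholds, player sight, recency of sighting and distance into StaminaLow, StaminaFull, IsSafe and PlayerTooClose flags.
; The flags are controller variables, with no Blackboard writes in this Blueprint.
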(event `self.ReceiveBeginPlay`
  (bind _returnvalue (`self.K2_GetPawn`))
  (bind _returnvalue_2 (`GameplayStatics.GetPlayerPawn` 0))
  (`/Engine/EditorBlueprintResources/StandardMacros.IsValid` _returnvalue
    (:`Is Valid`
      (bind _asbp_npcbt (cast `/Game/Dissertation/AI_NPC/BT/BP_NPCBT` _returnvalue))
      (set `self.BTNPC` _asbp_npcbt)
      (`/Engine/EditorBlueprintResources/StandardMacros.IsValid` _returnvalue_2
        (:`Is Valid`
          (bind _asbp_first_person_character (cast `/Game/FirstPerson/Blueprints/BP_FirstPersonCharacter` _returnvalue_2))
          (set `self.Player` _asbp_first_person_character))))))

(event `self.ReceivePossess`
  (params (PossessedPawn :type "Pawn Object Reference"))
  (`self.RunBehaviorTree` "/Game/Dissertation/BT/BT_NPCBehaviour.BT_NPCBehaviour"))

(event `self.ReceiveTick`
  (params (DeltaSeconds :type "Float (single-precision)"))
  (`self.UpdateBT`))

(fn `UpdateBT`
  (`|ExecutionSequence`
    (:`then_0`
      (if (<= (`/Game/Dissertation/AI_NPC/BT/BP_NPCBT.Stamina` (`self.BTNPC`)) 30.0)
        (set `self.StaminaLow` true)
        (else
          (set `self.StaminaLow` false))))
    (:`then_1`
      (if (>= (`/Game/Dissertation/AI_NPC/BT/BP_NPCBT.Stamina` (`self.BTNPC`)) 85.0)
        (set `self.StaminaFull` true)
        (else
          (set `self.StaminaFull` false))))
    (:`then_2`
      (if (and (`/Game/Dissertation/AI_NPC/BT/BP_NPCBT.CanSeePlayer` (`self.BTNPC`)) (<= (`KismetMathLibrary.Vector_Distance` (`SceneComponent.K2_GetComponentLocation` (`Character.CapsuleComponent` (`self.BTNPC`))) (`SceneComponent.K2_GetComponentLocation` (`Character.CapsuleComponent` (`self.Player`)))) 1000.0) (< (`/Game/Dissertation/AI_NPC/BT/BP_NPCBT.TimeSinceSawPlayer` (`self.BTNPC`)) 5.0))
        (set `self.IsSafe` false)
        (else
          (set `self.IsSafe` true))))
    (:`then_3`
      (if (< (`self.GetDistanceTo` (`self.BTNPC`) (`self.Player`)) 500.0)
        (set `self.PlayerTooClose` true)
        (else
          (set `self.PlayerTooClose` false))))))

(fn `UserConstructionScript`)